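; Space shooter enemy that spins continuously around its yaw axis, layered on parent enemy logic.
; BeginPlay sets MovementVector to forward plus a random sideways component.
; Overlapping a "Lateral"-tagged actor toggles IsRight and flips MovementVector between two opposite diagonals built from current actor axes.
; Every other such bounce, when IsRight turns false, also shortens DelayShot.
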(event EventBeginPlay
  (|CallParentFunction)
  (Variables|Default|SetMovementVector (+ (* (Transformation|GetActorRightVector) (Math|Random|RandomIntegerinRange -1 1)) (Transformation|GetActorForwardVector)))
  (Variables|Default|SetIsRight true))

(event Collision|EventActorBeginOverlap
  (params (OtherActor :type Actor%20Object%20Reference))
  (bind _returnvalue (Transformation|GetActorRightVector))
  (bind _returnvalue_2 (Transformation|GetActorForwardVector))
  (bind _returnvalue_3 (- _returnvalue _returnvalue_2))
  (|CallParentFunction OtherActor)
  (if (Utilities|Array|ContainsItem (Variables|/Script/Engine.Actor|GetTags OtherActor) "Lateral")
    (if (Variables|Default|GetIsRight)
      (Variables|Default|SetIsRight false)
      (Variables|Default|SetMovementVector (* _returnvalue_3 -1.0))
      (Variables|Default|SetDelayShot (- (Variables|Default|GetDelayShot) 0.1))
      (else
        (Variables|Default|SetIsRight true)
        (Variables|Default|SetMovementVector _returnvalue_3)))))

(event EventTick
  (params (DeltaSeconds :type Float%20%28single-precision%29))
  (|CallParentFunction DeltaSeconds)
  (Transformation|AddActorLocalRotation (* (Math|Rotator|MakeRotator 0.0 0.0 7e+01) DeltaSeconds) false false))

(fn ConstructionScript
  (|CallParentFunction))