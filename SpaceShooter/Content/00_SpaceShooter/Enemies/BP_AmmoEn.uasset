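; BP_AmmoEn is an enemy projectile for the space shooter.
; On Tick it moves along its forward vector by Speed, scaled by delta time and without sweep.
; On overlap it ignores BP_EnemyH and BP_EnemyBase actors; anything else triggers an explosion emitter and 2D sound, then destruction after a short delay.
; It applies no damage in its own graph.
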(event EventBeginPlay)

(event Collision|EventActorBeginOverlap
  (params (OtherActor :type Actor%20Object%20Reference))
  ;[1 1 1] Colisión Ammo
  (Utilities|Casting|CastToBP_EnemyH OtherActor
    (:CastFailed
      (Utilities|Casting|CastToBP_EnemyBase OtherActor
        (:CastFailed
          (Effects|SpawnEmitteratLocation "/Game/StarterContent/Particles/P_Explosion.P_Explosion" (Transformation|GetActorLocation)) ; Partículas
          (Audio|PlaySound2D "/Game/StarterContent/Audio/Explosion02.Explosion02" 1.0 1.0 0.0 0 0) ; Sonido
          (Utilities|FlowControl|Delay 0.2)
          (Actor|DestroyActor) ; Autodestruir
        )))))

(event EventTick
  (params (DeltaSeconds :type Float%20%28single-precision%29))
  ;[1 1 1] Actualizar posición
  (Transformation|SetActorLocation (+ (Transformation|GetActorLocation) (* (Transformation|GetActorForwardVector) (* DeltaSeconds (Variables|Default|GetSpeed)))) false false))

(fn ConstructionScript)